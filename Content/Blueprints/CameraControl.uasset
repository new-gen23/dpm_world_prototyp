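; CameraControl is a Blueprint that rotates the controller's view with yaw and pitch input while the right mouse button is held.
; Right mouse press and release events set the RightMouseButtonHeld flag, with release clearing it.
; Tick checks that flag and feeds axis values into AddControllerYawInput and AddControllerPitchInput.
; The PitchControl and YawControl axis events have empty execution bodies, so all rotation runs from Tick.
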(event EventBeginPlay)

(event Collision|EventActorBeginOverlap
  (params (OtherActor :type Actor%20Object%20Reference)))

(event EventTick
  (params (DeltaSeconds :type Float%20%28single-precision%29))
  (if (Variables|Default|GetRightMouseButtonHeld)
    (Pawn|Input|AddControllerYawInput (stale Input|AxisEvents|InputAxisYawControl AxisValue))
    (Pawn|Input|AddControllerPitchInput (stale Input|AxisEvents|InputAxisPitchControl AxisValue))))

(event Input|AxisEvents|InputAxisYawControl
  (params (AxisValue :type Float%20%28single-precision%29)))

(event Input|AxisEvents|InputAxisPitchControl
  (params (AxisValue :type Float%20%28single-precision%29)))

(event Input|MouseEvents|RightMouseButton
  (params (Key :type Key%20Structure :default "AnyKey"))
  (:Pressed
    (Variables|Default|SetRightMouseButtonHeld true))
  (:Released
    (Variables|Default|SetRightMouseButtonHeld false)))

(fn ConstructionScript)